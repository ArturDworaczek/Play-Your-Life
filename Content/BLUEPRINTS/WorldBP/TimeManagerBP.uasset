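; Time manager Blueprint that drives the day/night sky and announces switches between day and night, starting its cycle at noon on day zero.
; UpdateSunLocation rotates the Sun, offsets the Moon's pitch by 180 degrees and refreshes the sky's sun direction.
; When the world state changes, a DoOnce-gated branch sends Day or Night messages to all TimeManagerInterface actors and toggles the Sun's intensity within that loop.
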(event `self.ReceiveBeginPlay`
  (`self.StartCycle` 0 12.0))

(event `self.UpdateSunLocation`
  (params (SunRotation :type "Rotator Structure"))
  (bind _moon (`self.Moon`))
  (bind _sun (`self.Sun`))
  (bind _sun_2 (`self.Sun`))
  (bind _sun_3 (`self.Sun`))
  (`/Engine/EditorBlueprintResources/StandardMacros.IsValid` _sun_2
    (:`Is Valid`
      (`self.K2_SetActorRotation` _sun_2 SunRotation false))
    (:`Is Not Valid`
      _))
  (`/Engine/EditorBlueprintResources/StandardMacros.IsValid` _moon
    (:`Is Valid`
      (`self.K2_SetActorRotation` _moon (`KismetMathLibrary.MakeRotator` (.roll SunRotation) (+ (.pitch SunRotation) 180.0) (.yaw SunRotation)) false))
    (:`Is Not Valid`
      _))
  (`/Game/BLUEPRINTS/WorldBP/Sky/Sky.UpdateSunDirection` (`self.Sky`))
  (if (`|EnumInequality` (`self.CurrentWorldState`) (`self.CurrentState`))
    (`|ExecutionSequence`
      (:`then_0`
        (goto _label :!via `Reset`))
      (:`then_1`
        (`/Engine/EditorBlueprintResources/StandardMacros.DoOnce` true :!label _label
          (:`Completed`
            (if (`|EnumEquality` (`self.CurrentWorldState`) "E_Day")
              (set `self.CurrentState` "E_Day")
              (bind _outactors (`GameplayStatics.GetAllActorsWithInterface` "/Game/BLUEPRINTS/WorldBP/TimeManagerInterface.TimeManagerInterface_C"))
              (for _array_element _outactors
                (message `/Game/BLUEPRINTS/WorldBP/TimeManagerInterface.Day` _array_element)
                (`/Engine/EditorBlueprintResources/StandardMacros.IsValid` _sun_3
                  (:`Is Valid`
                    (`LightComponent.SetIntensity` (`Light.LightComponent` _sun_3) 1.5))))
              (else
                (set `self.CurrentState` "E_Night")
                (bind _outactors_2 (`GameplayStatics.GetAllActorsWithInterface` "/Game/BLUEPRINTS/WorldBP/TimeManagerInterface.TimeManagerInterface_C"))
                (for _array_element_2 _outactors_2
                  (message `/Game/BLUEPRINTS/WorldBP/TimeManagerInterface.Night` _array_element_2)
                  (`/Engine/EditorBlueprintResources/StandardMacros.IsValid` _sun
                    (:`Is Valid`
                      (`LightComponent.SetIntensity` (`Light.LightComponent` _sun) 0.0))))))))))))

(fn `UserConstructionScript`)