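; Door is a placeable hinged door Blueprint that swings open and closed through OpenDoor and CloseDoor events.
; Each event plays one of two timelines, chosen by the Invert flag for swing direction, which drive the static mesh's relative yaw.
; An AnimPlaying flag ignores new requests mid-swing, while DoorOpen records the state.
; The construction script applies the mesh from the Door variable.
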(event `self.OpenDoor`
  (if (not (`self.bAnimPlaying`))
    (set `self.bDoorOpen` true)
    (if (`self.bInvert`)
      (set `self.bAnimPlaying` true)
      (bind (_direction _doorturn) (`Timeline|DoorOpenOut` :!via `PlayFromStart`)
        (:`Update`
          (`SceneComponent.K2_SetRelativeRotation` (`self.StaticMesh`) (`KismetMathLibrary.MakeRotator` 0.0 0.0 _doorturn) false false))
        (:`Finished`
          (set `self.bAnimPlaying` false)))
      (else
        (set `self.bAnimPlaying` true)
        (bind (_direction_2 _doorturn_2) (`Timeline|DoorOpenIn` :!via `PlayFromStart`)
          (:`Update`
            (`SceneComponent.K2_SetRelativeRotation` (`self.StaticMesh`) (`KismetMathLibrary.MakeRotator` 0.0 0.0 _doorturn_2) false false))
          (:`Finished`
            (set `self.bAnimPlaying` false)))))))

(event `self.CloseDoor`
  (if (not (`self.bAnimPlaying`))
    (set `self.bDoorOpen` false)
    (if (`self.bInvert`)
      (set `self.bAnimPlaying` true)
      (bind (_direction _doorturn) (`Timeline|CloseDoorOut` :!via `PlayFromStart`)
        (:`Update`
          (`SceneComponent.K2_SetRelativeRotation` (`self.StaticMesh`) (`KismetMathLibrary.MakeRotator` 0.0 0.0 _doorturn) false false))
        (:`Finished`
          (set `self.bAnimPlaying` false)))
      (else
        (set `self.bAnimPlaying` true)
        (bind (_direction_2 _doorturn_2) (`Timeline|CloseDoorIn` :!via `PlayFromStart`)
          (:`Update`
            (`SceneComponent.K2_SetRelativeRotation` (`self.StaticMesh`) (`KismetMathLibrary.MakeRotator` 0.0 0.0 _doorturn_2) false false))
          (:`Finished`
            (set `self.bAnimPlaying` false)))))))

(fn `UserConstructionScript`
  (`StaticMeshComponent.SetStaticMesh` (`self.StaticMesh`) (`self.Door`)))