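; Player controller that handles gesture, pause menu, player list and chat input.
; Gesture keys send animations to server functions, or return to the animation Blueprint if one is playing.
; HUD toggles, chat updates colored by account type and notifications route through PYLHUD's main widget, while pause opens a UI-only menu.
; BeginPlay calls GetActionKeys, and UpdateActionKey events add mappings to the game instance.
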(event `self.ReceiveBeginPlay`
  ;[1 1 1] BeginPlay
  (`self.GetActionKeys`))

(event `self.CallReturnToAnimBP`
  ;[1 1 1] Show Gestures Menu
  (`self.ReturnToAnimationBP`))

(event `InputAction|Gesture 1`
  (params (Key :type "Key Structure"))
  ;[1 1 1] Show Gestures Menu
  (:`Pressed`
    (`self.PlayGesture` 0)))

(event `InputAction|Gesture 2`
  (params (Key :type "Key Structure"))
  ;[1 1 1] Show Gestures Menu
  (:`Pressed`
    (`self.PlayGesture` 1)))

(event `InputAction|Gesture 3`
  (params (Key :type "Key Structure"))
  ;[1 1 1] Show Gestures Menu
  (:`Pressed`
    (`self.PlayGesture` 2)))

(event `InputAction|Gesture 4`
  (params (Key :type "Key Structure"))
  ;[1 1 1] Show Gestures Menu
  (:`Pressed`
    (`self.PlayGesture` 3)))

(event `InputAction|PauseMenu`
  (params (Key :type "Key Structure"))
  ;[1 1 1] Show PauseMenu
  (:`Pressed`
    (bind _returnvalue (`|CreateWidget` "/Game/UIBLUEPRINTS/PauseMenu/MenuUI.MenuUI_C" self))
    (bind _output_get (set `self.PauseMenu` _returnvalue))
    (`UserWidget.AddToViewport` _output_get 99)
    (`WidgetBlueprintLibrary.SetInputMode_UIOnlyEx` self _output_get)
    (set `self.bShowMouseCursor` true)))

(event `InputAction|TogglePlayerList`
  (params (Key :type "Key Structure"))
  ;[1 1 1] Toggle Playerlist
  (:`Pressed`
    (`/Engine/EditorBlueprintResources/StandardMacros.DoOnce` false :!label _label
      (:`Completed`
        (bind _aspylhud (cast `/Game/BLUEPRINTS/GamemodeBP/PYLHUD` (`self.GetHUD`)))
        (`/Engine/EditorBlueprintResources/StandardMacros.FlipFlop`
          (:`A`
            (bind _mainhud (`/Game/BLUEPRINTS/GamemodeBP/PYLHUD.MAINHUD` _aspylhud))
            (`/Game/UIBLUEPRINTS/MAINHUD/MAINHUD.Show Playerlist` _mainhud))
          (:`B`
            (`/Game/UIBLUEPRINTS/MAINHUD/MAINHUD.Hide Playerlist` _mainhud)))
        (`KismetSystemLibrary.Delay` 1.0)
        (goto _label :!via `Reset`)))))

(event `InputAction|Chat`
  (params (Key :type "Key Structure"))
  ;[1 1 1] Chat
  (:`Pressed`
    (bind _aspylhud (cast `/Game/BLUEPRINTS/GamemodeBP/PYLHUD` (`self.GetHUD`)))
    (`/Engine/EditorBlueprintResources/StandardMacros.FlipFlop`
      (:`A`
        (bind _mainhud (`/Game/BLUEPRINTS/GamemodeBP/PYLHUD.MAINHUD` _aspylhud))
        (`/Game/UIBLUEPRINTS/MAINHUD/MAINHUD.ShowChatbox` _mainhud)
        (`/Game/UIBLUEPRINTS/MAINHUD/MAINHUD.Hide Playerlist` _mainhud))
      (:`B`
        (`/Game/UIBLUEPRINTS/MAINHUD/MAINHUD.HideChatBox` _mainhud)))))

(event `self.UpdateChat`
  (params (Message :type "ChatMessage Structure") (Colour :type "EAccountType Enum" :default "AT_Normal"))
  (bind (_normalaccount _premiumaccount _premiumplusaccount _helperaccount _modaccount _adminaccount) (`self.GetAccountTypeColour`))
  ;[1 1 1] Chat
  ;;[1 1 1] Chat Updating
  (`self.UpdateChatBP` Message (select `EAccountType` Colour :`AT_Normal` _normalaccount :`AT_Premium` _premiumaccount :`AT_PremiumPlus` _premiumplusaccount :`AT_Helper` _helperaccount :`AT_Moderator` _modaccount :`AT_Admin` _adminaccount)))

(event `UpdateChatBP`
  (params (MessageInfo :type "ChatMessage Structure") (AccountColour :type "SlateColor Structure"))
  ;[1 1 1] Chat
  ;;[1 1 1] Chat Updating
  (bind _aspylhud (cast `/Game/BLUEPRINTS/GamemodeBP/PYLHUD` (`self.GetHUD`)))
  (`/Game/UIBLUEPRINTS/MAINHUD/MAINHUD.UpdateChat` (`/Game/BLUEPRINTS/GamemodeBP/PYLHUD.MAINHUD` _aspylhud) MessageInfo AccountColour))

(event `self.UpdateNotification`
  (params (Notification :type "Notification Structure"))
  (bind (_player _notification _amount _from _sender) (break `Notification` Notification))
  ;[1 1 1] Notification
  (`self.UpdateNotificationBP` (not (`self.bNotifPlaying`)) _player _notification _amount _from _sender))

(event `UpdateNotificationBP`
  (params (bNotifPlaying :type Boolean) (Player :type String) (Notification :type String) (Amount :type String) (From :type String) (Sender :type String))
  ;[1 1 1] Notification
  (if bNotifPlaying
    (bind _aspylhud (cast `/Game/BLUEPRINTS/GamemodeBP/PYLHUD` (`self.GetHUD`)))
    (`/Game/UIBLUEPRINTS/MAINHUD/MAINHUD.SendNotification` (`/Game/BLUEPRINTS/GamemodeBP/PYLHUD.MAINHUD` _aspylhud) (`KismetTextLibrary.Conv_StringToText` Player) (`KismetTextLibrary.Conv_StringToText` Notification) (`KismetTextLibrary.Conv_StringToText` Amount) (`KismetTextLibrary.Conv_StringToText` From) (`KismetTextLibrary.Conv_StringToText` Sender))))

(event `self.UpdateActionKey`
  (params (ActionKeyInformation :type "InputActionKeyMapping Structure"))
  ;[1 1 1] ActionKeys
  (bind _aspylgame_instance (cast `/Game/BLUEPRINTS/GamemodeBP/PYLGameInstance` (`GameplayStatics.GetGameInstance`)))
  (`KismetArrayLibrary.Array_Add` (`/Game/BLUEPRINTS/GamemodeBP/PYLGameInstance.ActionMappings` _aspylgame_instance) ActionKeyInformation))

(fn `GetAccountTypeColour`
  (returns (NormalAccount :type "SlateColor Structure") (PremiumAccount :type "SlateColor Structure") (PremiumPlusAccount :type "SlateColor Structure") (HelperAccount :type "SlateColor Structure") (ModAccount :type "SlateColor Structure") (AdminAccount :type "SlateColor Structure"))
  (return (make `SlateColor` (struct :`A` 1.0)) (make `SlateColor` (struct :`G` 0.036073 :`B` 1.0 :`A` 1.0)) (make `SlateColor` (struct :`R` 1.0 :`G` 0.917489 :`A` 1.0)) (make `SlateColor` (struct :`G` 1.0 :`A` 1.0)) (make `SlateColor` (struct :`R` 1.0 :`G` 0.436026 :`A` 1.0)) (make `SlateColor` (struct :`R` 1.0 :`A` 1.0))))

(fn `PlayGesture`
  (params (Index :type Integer))
  (if (`self.bGesturePlaying`)
    (`self.ReturnToAnimationBP`)
    (else
      (`self.PlayGestureOnServer` (`self.K2_GetPawn`) (`|GetArrayItem` (`self.Gestures`) Index)))))

(fn `ReturnToAnimationBP`
  (`self.ReturnToAnimBPServer` (`self.K2_GetPawn`) "/Game/CHARACTER/MAN/Animations/ANIMATION_BP.ANIMATION_BP_C")
  (`self.SetbGesturePlaying` false))

(fn `UserConstructionScript`)