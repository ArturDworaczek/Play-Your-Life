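; Game instance that holds the player's options (master, music, SFX and voice chat volumes, plus action mappings) and persists them to disk.
; SaveOptions copies the values into a new OptionsSave object and writes it to the UserSettings slot.
; LoadOptions reads that slot back into its variables, replacing action mappings only when the saved list is non-empty.
; It only stores the values and does not apply them to audio or input.
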(event `SaveOptions`
  (bind _returnvalue (`GameplayStatics.CreateSaveGameObject` "/Game/BLUEPRINTS/GamemodeBP/Save/OptionsSave.OptionsSave_C"))
  (bind _asoptions_save (cast `/Game/BLUEPRINTS/GamemodeBP/Save/OptionsSave` _returnvalue))
  (bind _output_get (set `self.OptionsData` _asoptions_save))
  (set `/Game/BLUEPRINTS/GamemodeBP/Save/OptionsSave.MasterVolume` (`self.MasterVolume`) _output_get)
  (set `/Game/BLUEPRINTS/GamemodeBP/Save/OptionsSave.MusicVolume` (`self.MusicVolume`) _output_get)
  (set `/Game/BLUEPRINTS/GamemodeBP/Save/OptionsSave.SFXVolume` (`self.SFXVolume`) _output_get)
  (set `/Game/BLUEPRINTS/GamemodeBP/Save/OptionsSave.VoiceChatVolume` (`self.VoiceChatVolume`) _output_get)
  (set `/Game/BLUEPRINTS/GamemodeBP/Save/OptionsSave.ActionMappings` (`self.ActionMappings`) _output_get)
  (`GameplayStatics.SaveGameToSlot` (`self.OptionsData`) "UserSettings"))

(event `LoadOptions`
  (bind _returnvalue (`GameplayStatics.CreateSaveGameObject` "/Game/BLUEPRINTS/GamemodeBP/Save/OptionsSave.OptionsSave_C"))
  (bind _asoptions_save (cast `/Game/BLUEPRINTS/GamemodeBP/Save/OptionsSave` _returnvalue))
  (set `self.OptionsData` _asoptions_save)
  (bind _returnvalue_2 (`GameplayStatics.LoadGameFromSlot` "UserSettings"))
  (bind _asoptions_save_2 (cast `/Game/BLUEPRINTS/GamemodeBP/Save/OptionsSave` _returnvalue_2))
  (set `self.MasterVolume` (`/Game/BLUEPRINTS/GamemodeBP/Save/OptionsSave.MasterVolume` _asoptions_save_2))
  (set `self.SFXVolume` (`/Game/BLUEPRINTS/GamemodeBP/Save/OptionsSave.SFXVolume` _asoptions_save_2))
  (set `self.MusicVolume` (`/Game/BLUEPRINTS/GamemodeBP/Save/OptionsSave.MusicVolume` _asoptions_save_2))
  (set `self.VoiceChatVolume` (`/Game/BLUEPRINTS/GamemodeBP/Save/OptionsSave.VoiceChatVolume` _asoptions_save_2))
  (bind _actionmappings (`/Game/BLUEPRINTS/GamemodeBP/Save/OptionsSave.ActionMappings` _asoptions_save_2))
  (if (> (`KismetArrayLibrary.Array_Length` _actionmappings) 0)
    (`KismetArrayLibrary.Array_Clear` (`self.ActionMappings`))
    (set `self.ActionMappings` _actionmappings)))