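; Configurable path light prop that switches between a tall and a small lamp variant through the TallSmall flag.
; The construction script shows the chosen mesh and point light, hides the other pair, and hides a "Do First" billboard.
; A dynamic material instance shares color and intensity between the lamp's emissive and its light.
; The small variant derives a dimmer intensity and shorter attenuation radius from the same settings.
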(fn `UserConstructionScript`
  ;[1 0.3451 0] check the box to hide the do First message
  (set `self.HIDE_DoFirstBillboard` true)
  (if (`self.HIDE_DoFirstBillboard`)
    (`SceneComponent.SetVisibility` (`self.Do First Billboard`) false false))
  (`SceneComponent.SetVisibility` (`self.Tall Lamp`) (not (`self.Tall/Small`)) false)
  (`SceneComponent.SetVisibility` (`self.PointLightTall`) (not (`self.Tall/Small`)) false)
  (`SceneComponent.SetVisibility` (`self.Small lamp`) (`self.Tall/Small`) false)
  (`SceneComponent.SetVisibility` (`self.PointLightSmall`) (`self.Tall/Small`) false)
  (if (`self.Tall/Small`)
    (bind _returnvalue (`PrimitiveComponent.CreateDynamicMaterialInstance` (`self.Small lamp`) 0 null))
    (set `self.DMI` _returnvalue)
    (`LightComponent.SetLightColor` (`self.PointLightSmall`) (`self.Light Color`) (`self.sRGB`))
    (`LightComponent.SetIntensity` (`self.PointLightSmall`) (/ (* (`self.L+E Intensity`) (`self.Light Multiplier`)) 8.0))
    (`MaterialInstanceDynamic.SetVectorParameterValue` (`self.DMI`) "Emissive Color" (`self.Light Color`))
    (`MaterialInstanceDynamic.SetScalarParameterValue` (`self.DMI`) "Emissive Intensity" (`self.L+E Intensity`))
    (`PointLightComponent.SetAttenuationRadius` (`self.PointLightSmall`) (- (`self.Attenuationradius`) 158.0))
    (`LightComponent.SetIndirectLightingIntensity` (`self.PointLightSmall`) (`self.Indirect Light Intensity`))
    (else
      (bind _returnvalue_2 (`PrimitiveComponent.CreateDynamicMaterialInstance` (`self.Tall Lamp`) 0 null))
      (set `self.DMI` _returnvalue_2)
      (`LightComponent.SetLightColor` (`self.PointLightTall`) (`self.Light Color`) (`self.sRGB`))
      (`LightComponent.SetIntensity` (`self.PointLightTall`) (* (`self.L+E Intensity`) (`self.Light Multiplier`)))
      (`MaterialInstanceDynamic.SetVectorParameterValue` (`self.DMI`) "Emissive Color" (`self.Light Color`))
      (`MaterialInstanceDynamic.SetScalarParameterValue` (`self.DMI`) "Emissive Intensity" (`self.L+E Intensity`))
      (`PointLightComponent.SetAttenuationRadius` (`self.PointLightTall`) (`self.Attenuationradius`))
      (`LightComponent.SetIndirectLightingIntensity` (`self.PointLightTall`) (`self.Indirect Light Intensity`)))))