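; Path light prop Blueprint that pairs a static mesh with a point light, both configured from shared variables.
; The construction script sets the light's color, intensity, attenuation radius and indirect lighting intensity.
; It also creates a dynamic material instance on the mesh and drives its emissive color and intensity from the same color and intensity values, with a multiplier applied only to the light.
; The event graph holds no active logic.
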(fn `UserConstructionScript`
  (bind _returnvalue (`PrimitiveComponent.CreateDynamicMaterialInstance` (`self.StaticMesh`) 0 null))
  (set `self.DMI` _returnvalue)
  (`LightComponent.SetLightColor` (`self.PointLight`) (`self.LightColor`) (`self.sRGB`))
  (`LightComponent.SetIntensity` (`self.PointLight`) (* (`self.L+E Intensity`) (`self.Light Multiplier`)))
  (`PointLightComponent.SetAttenuationRadius` (`self.PointLight`) (`self.Attenuation Radius`))
  (`LightComponent.SetIndirectLightingIntensity` (`self.PointLight`) (`self.Indirect Lighting Intensity`))
  (`MaterialInstanceDynamic.SetVectorParameterValue` (`self.DMI`) "Emissive Color" (`self.LightColor`))
  (`MaterialInstanceDynamic.SetScalarParameterValue` (`self.DMI`) "Emissive Intensity" (`self.L+E Intensity`)))