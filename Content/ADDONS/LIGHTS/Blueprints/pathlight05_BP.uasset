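; Path light Blueprint with a point light and an emissive mesh, switchable between hard-edge and round-edge variants.
; The construction script picks the visible mesh, creates its dynamic material, applies light color, intensity, radius and indirect lighting, and calls the flicker events.
; Flicker, marked test-only, uses a gated loop with random delays to toggle light visibility.
; Day and Night events zero or restore light and emissive intensity.
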(event `FlickerTRUE`
  ;[0 0 0] for test purpose only
  (`MaterialInstanceDynamic.SetScalarParameterValue` (`self.DMI`) "Emissive Intensity" 0.0)
  (`|ExecutionSequence`
    (:`then_0`
      (goto _label :!via `Open`))
    (:`then_1`
      (`/Engine/EditorBlueprintResources/StandardMacros.Gate` true :!label _label
        (:`Exit`
          (`|ExecutionSequence`
            (:`then_0`
              (`SceneComponent.SetVisibility` (`self.PointLight`) false false))
            (:`then_1`
              (`KismetSystemLibrary.Delay` (`KismetMathLibrary.RandomFloatInRange` 0.01 0.47))
              (`SceneComponent.SetVisibility` (`self.PointLight`) true false)
              (`MaterialInstanceDynamic.SetScalarParameterValue` (`self.DMI`) "Emissive Intensity" (`self.L+E Intensity`))
              (goto _label))))))))

(event `FlickerFALSE`
  ;[0 0 0] for test purpose only
  (goto _label :!via `Close`))

(event `/Game/BLUEPRINTS/WorldBP/TimeManagerInterface.Day`
  ;[0 0 0] for test purpose only
  (`LightComponent.SetIntensity` (`self.PointLight`) 0.0)
  (`MaterialInstanceDynamic.SetScalarParameterValue` (`self.DMI`) "Emissive Intensity" 0.0))

(event `/Game/BLUEPRINTS/WorldBP/TimeManagerInterface.Night`
  (bind _l_e_intensity (`self.L+E Intensity`))
  ;[0 0 0] for test purpose only
  (`LightComponent.SetIntensity` (`self.PointLight`) (* (`self.Light Multiplier`) _l_e_intensity))
  (`MaterialInstanceDynamic.SetScalarParameterValue` (`self.DMI`) "Emissive Intensity" _l_e_intensity))

(fn `UserConstructionScript`
  (if (`self.Flickering`)
    (`self.FlickerTRUE`)
    (else
      (`self.FlickerFALSE`)))
  (`SceneComponent.SetVisibility` (`self.HardEdge`) (not (`self.Round/Hard edge`)) false)
  (`SceneComponent.SetVisibility` (`self.StaticMesh`) (`self.Round/Hard edge`) false)
  (if (`self.Round/Hard edge`)
    ;[0 0 0] round edge mat
    (bind _returnvalue (`PrimitiveComponent.CreateDynamicMaterialInstance` (`self.StaticMesh`) 0 null))
    (set `self.DMI` _returnvalue)
    (else
      ;[0 0 0] hard edge mat
      (bind _returnvalue_2 (`PrimitiveComponent.CreateDynamicMaterialInstance` (`self.HardEdge`) 0 null))
      (set `self.DMI` _returnvalue_2)))
  (`LightComponent.SetLightColor` (`self.PointLight`) (`self.LightColor`) (`self.sRGB`))
  (`LightComponent.SetIntensity` (`self.PointLight`) (* (`self.L+E Intensity`) (`self.Light Multiplier`)))
  (`PointLightComponent.SetAttenuationRadius` (`self.PointLight`) (`self.Attenuation Radius`))
  (`LightComponent.SetIndirectLightingIntensity` (`self.PointLight`) (`self.Indirect Lighting Intesity`))
  (`MaterialInstanceDynamic.SetVectorParameterValue` (`self.DMI`) "Emissive Color" (`self.LightColor`))
  (`MaterialInstanceDynamic.SetScalarParameterValue` (`self.DMI`) "Emissive Intensity" (`self.L+E Intensity`)))